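; Door actor that swings open and closed by yaw rotation each time its Trigger event is called.
; A DoorRotation timeline plays or reverses based on the Closed flag, while a Moving flag ignores triggers mid-swing.
; When the timeline finishes, it flips Closed, prints a debug message and, if AutoClose is set, starts a timer that calls Trigger again to shut the opened door.
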(event `Event Trigger`
  (if (not (`self.Moving`))
    (set `self.Moving` true)
    (if (`self.Closed`)
      (bind (_direction _doorrot) (`Timeline|DoorRotation` :!label _label)
        (:`Update`
          (`SceneComponent.K2_SetRelativeRotation` (`self.Door`) (`KismetMathLibrary.MakeRotator` 0.0 0.0 _doorrot) false false))
        (:`Finished`
          (set `self.Closed` (not (`self.Closed`)))
          (set `self.Moving` false)
          (`KismetSystemLibrary.PrintText` "stopped")
          (if (`self.AutoClose`)
            (if (not (`self.Closed`))
              (`KismetSystemLibrary.K2_SetTimerDelegate` (delegate `Event Trigger`) (`self.AutoClose_time`))))))
      (else
        (goto _label :!via `Reverse`)))))

(event `self.ReceiveBeginPlay`)

(event `self.ReceiveTick`
  (params (DeltaSeconds :type "Float (single-precision)")))

(fn `UserConstructionScript`)