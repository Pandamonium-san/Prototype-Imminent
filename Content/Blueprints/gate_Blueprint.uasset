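; Sewer gate actor whose trigger overlap acts only while the referenced sewer wheel is not drained.
; An overlapping player character reloads or opens FirstPersonExampleMap.
; An overlapping actor with a boulderfall component destroys the gate and plays a metal impact sound.
; The sound location comes from casting the overlapping actor to gate_Blueprint, not from the gate itself.
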(event `self.gate trigger.OnComponentBeginOverlap`
  (params (OverlappedComponent :type "PrimitiveComponent Object Reference") (OtherActor :type "Actor Object Reference") (OtherComp :type "PrimitiveComponent Object Reference") (OtherBodyIndex :type Integer) (bFromSweep :type Boolean) (SweepResult :type "HitResult Structure (by ref)"))
  (bind _assewer_wheel (cast `/Game/Blueprints/sewer_wheel` (`self.sewer_wheel`)))
  (if (not (`/Game/Blueprints/sewer_wheel.isDrained` _assewer_wheel))
    (cast `/Game/FirstPersonBP/Blueprints/interact_character` OtherActor
      (:`then`
        (`GameplayStatics.OpenLevel` "FirstPersonExampleMap"))
      (:`CastFailed`
        (`/Engine/EditorBlueprintResources/StandardMacros.IsValid` (`self.GetComponentByClass` OtherActor "/Game/Interact_boulderfall.Interact_boulderfall_C")
          (:`Is Valid`
            (bind _asgate_blueprint (cast `/Game/Blueprints/gate_Blueprint` OtherActor)
              (:`then`
                _)
              (:`CastFailed`
                _))
            (`self.K2_DestroyActor`)
            (`KismetSystemLibrary.PrintText` "boom")
            (`GameplayStatics.PlaySoundAtLocation` "/Game/Sounds/Metal_Impact_Sound_Effect.Metal_Impact_Sound_Effect" (`self.K2_GetActorLocation` _asgate_blueprint) (struct) 0.2))
          (:`Is Not Valid`
            (`KismetSystemLibrary.PrintText` "no boom")))))))

(fn `UserConstructionScript`)