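; Ladder actor that lets the interact_character climb by switching its movement mode inside a trigger volume.
; When the character's capsule enters LadderVolume, its movement is set to Flying, and when it leaves, back to Walking.
; Casts on both the actor and component limit the switch to that capsule, and debug text prints on each change.
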(event `self.LadderVolume.OnComponentBeginOverlap`
  (params (OverlappedComponent :type "PrimitiveComponent Object Reference") (OtherActor :type "Actor Object Reference") (OtherComp :type "PrimitiveComponent Object Reference") (OtherBodyIndex :type Integer) (bFromSweep :type Boolean) (SweepResult :type "HitResult Structure (by ref)"))
  (bind _asinteract_character (cast `/Game/FirstPersonBP/Blueprints/interact_character` OtherActor))
  (cast `CapsuleComponent` OtherComp)
  (`CharacterMovementComponent.SetMovementMode` (`Character.CharacterMovement` _asinteract_character) "MOVE_Flying" 0)
  (`KismetSystemLibrary.PrintText` "on"))

(event `self.LadderVolume.OnComponentEndOverlap`
  (params (OverlappedComponent :type "PrimitiveComponent Object Reference") (OtherActor :type "Actor Object Reference") (OtherComp :type "PrimitiveComponent Object Reference") (OtherBodyIndex :type Integer))
  (bind _asinteract_character (cast `/Game/FirstPersonBP/Blueprints/interact_character` OtherActor))
  (cast `CapsuleComponent` OtherComp)
  (`CharacterMovementComponent.SetMovementMode` (`Character.CharacterMovement` _asinteract_character) "MOVE_Walking" 0)
  (`KismetSystemLibrary.PrintText` "off"))

(fn `UserConstructionScript`)