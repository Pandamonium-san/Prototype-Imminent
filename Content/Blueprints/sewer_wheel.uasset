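; Sewer wheel actor that toggles a set of SewerWater actors between drained and undrained when triggered.
; BeginPlay caches each water actor's location as the base position.
; Trigger plays or reverses a timeline that offsets each actor's height from that base and scales its water sound volume.
; A Draining flag ignores triggers mid-animation, and IsDrained flips on completion to choose the next direction.
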(event `self.ReceiveBeginPlay`
  (for (_array_element _array_index) (`self.sewer_water`)
    (`KismetArrayLibrary.Array_Set` (`self.sewer_water_pos`) _array_index (`self.K2_GetActorLocation` _array_element) true)))

(event `Event Trigger`
  (if (not (`self.draining`))
    (set `self.draining` true)
    (`KismetSystemLibrary.PrintText` "drain")
    (if (`self.isDrained`)
      (bind (_direction _waterdrain _watervolme) (`Timeline|Timeline_waterdrain` :!via `ReverseFromEnd` :!label _label)
        (:`Update`
          (for (_array_element _array_index) (`self.sewer_water`)
            (`self.K2_SetActorLocation` _array_element (+ (`KismetArrayLibrary.Array_Get` (`self.sewer_water_pos`) _array_index) (`KismetMathLibrary.MakeVector` 0.0 0.0 _waterdrain)) false false)
            (bind _assewer_water (cast `/Game/SewerWater` _array_element))
            (`AudioComponent.SetVolumeMultiplier` (`/Game/SewerWater.waterSound` _assewer_water) _watervolme)))
        (:`Finished`
          (set `self.draining` false)
          (set `self.isDrained` (not (`self.isDrained`)))
          (`KismetSystemLibrary.PrintText` "drained")))
      (else
        (goto _label :!via `PlayFromStart`)))))

(fn `UserConstructionScript`)